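; BP_GameManagerBase is a base actor for game manager Blueprints that take part in saving and loading.
; On BeginPlay it caches the GI_Core game instance and binds to its prepare-save and save-loaded events, forwarding each to an empty hook function, apparently for child classes to override.
; Helpers validate and return the game instance's save game reference and print debug messages prefixed with the manager's display name.
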(event `self.ReceiveBeginPlay`
  (bind _asgi_core (cast `/Game/TrainGame/Core/GI_Core` (`GameplayStatics.GetGameInstance`)))
  (bind _output_get (set `self.GameInstanceRef` _asgi_core))
  (add `/Game/TrainGame/Core/GI_Core.OnPrepareSave` _output_get (delegate `OnPrepareSave_Handler`))
  (add `/Game/TrainGame/Core/GI_Core.OnSaveLoaded` _output_get (delegate `OnSaveLoaded_Handler`)))

(event `OnPrepareSave_Handler`
  (`self.OnPrepareSave_Event`))

(event `OnSaveLoaded_Handler`
  (`self.OnSaveLoad_Event`))

(fn `OnPrepareSave_Event`)

(fn `OnSaveLoad_Event`)

(fn `PrintMessage`
  (params (`In String` :type String) (TextColor :type "LinearColor Structure"))
  (`KismetSystemLibrary.PrintString` (`KismetStringLibrary.Concat_StrStr` (`KismetSystemLibrary.GetDisplayName` self) ": " `In String`) true true TextColor))

(fn `UserConstructionScript`)

(fn `ValidateGameInstanceAndSaveGame`
  (returns (SaveGameRef :type "/Game/TrainGame/Core/SaveGame/SG_GameData Object Reference"))
  (bind _gameinstanceref (`self.GameInstanceRef`))
  (bind _savegameref (`/Game/TrainGame/Core/GI_Core.SaveGameRef` _gameinstanceref))
  (`/Engine/EditorBlueprintResources/StandardMacros.IsValid` _gameinstanceref
    (:`Is Valid`
      (`/Engine/EditorBlueprintResources/StandardMacros.IsValid` _savegameref
        (:`Is Valid`
          (return _savegameref))
        (:`Is Not Valid`
          (`self.PrintMessage` "Save Game Ref Invalid!" (struct :`R` 1.0 :`A` 1.0)))))
    (:`Is Not Valid`
      (`self.PrintMessage` "Game Instance Ref Invalid!" (struct :`R` 1.0 :`A` 1.0)))))