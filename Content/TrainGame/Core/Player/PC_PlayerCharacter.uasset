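; Player controller for the train game's player character, owning the in-game menu and the switch between play and menu input.
; On BeginPlay it caches the GI_Core game instance and, if that cast succeeds, creates the WBP_Menu widget once.
; ToggleMenuVisibility adds or removes that widget, swapping between Game-and-UI input with a locked mouse and Game-only input, and matches cursor visibility to the menu state.
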(event `self.ReceiveBeginPlay`
  (bind _asgi_core (cast `/Game/TrainGame/Core/GI_Core` (`GameplayStatics.GetGameInstance`)))
  (set `self.Game Instance Ref` _asgi_core)
  (bind _returnvalue (`|CreateWidget` "/Game/TrainGame/Core/UI/WBP_Menu.WBP_Menu_C"))
  (set `self.MenuWidgetRef` _returnvalue))

(fn `Toggle Menu Visibility`
  (params (`Show Mouse Cursor` :type Boolean))
  (returns (`MenuOpen?` :type Boolean))
  (bind _menuwidgetref (`self.MenuWidgetRef`))
  (bind _bismenuopen (`self.bIsMenuOpen`))
  (`/Engine/EditorBlueprintResources/StandardMacros.IsValid` _menuwidgetref
    (:`Is Valid`
      (if (`self.bIsMenuOpen`)
        (`Widget.RemoveFromParent` _menuwidgetref)
        (`WidgetBlueprintLibrary.SetInputMode_GameOnly` self)
        (set `self.bIsMenuOpen` false)
        (`WidgetBlueprintLibrary.SetFocusToGameViewport`)
        (else
          (`UserWidget.AddToViewport` _menuwidgetref 0)
          (`WidgetBlueprintLibrary.SetInputMode_GameAndUIEx` self _menuwidgetref "LockAlways" false)
          (set `self.bIsMenuOpen` true)))
      (set `self.bShowMouseCursor` _bismenuopen)
      (return _bismenuopen))))

(fn `UserConstructionScript`)