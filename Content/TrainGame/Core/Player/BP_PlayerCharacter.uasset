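; First-person-style player character for a train game that walks, looks, jumps and places track segments.
; A camera line trace runs every tick, with debug drawing, to store the aimed-at location.
; The grab input toggles building: one trigger spawns a BP_TrackSegment just above that location, the next registers it with the tagged TrackManager found at BeginPlay.
; Enhanced Input mapping is added through PC_PlayerCharacter on BeginPlay.
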(event `self.ReceiveBeginPlay`
  (`|ExecutionSequence`
    (:`then_0`
      (`self.SetupInputSystem`))
    (:`then_1`
      (bind _outactors (`GameplayStatics.GetAllActorsWithTag` "TrackManager"))
      (bind _asbp_track_manager (cast `/Game/TrainGame/Core/Track/BP_TrackManager` (`|GetArrayItem` _outactors)))
      (set `self.TrackManagerRef` _asbp_track_manager))))

(event `EnhancedInput|/Game/TrainGame/Core/Player/Input/IA_Move`
  (params (ActionValue :type "Vector2D Structure") (ElapsedSeconds :type "Float (double-precision)") (TriggeredSeconds :type "Float (double-precision)") (InputAction :type "InputAction Object Reference" :default "/Game/TrainGame/Core/Player/Input/IA_Move.IA_Move"))
  (bind (_returnvalue_roll _returnvalue_pitch _returnvalue_yaw) (`KismetMathLibrary.BreakRotator` (`self.GetControlRotation`)))
  (bind (_returnvalue_roll_2 _returnvalue_pitch_2 _returnvalue_yaw_2) (`KismetMathLibrary.BreakRotator` (`self.GetControlRotation`)))
  (:`Triggered`
    (`self.AddMovementInput` (`KismetMathLibrary.GetRightVector` (`KismetMathLibrary.MakeRotator` _returnvalue_roll 0.0 _returnvalue_yaw)) ActionValue_X)
    (`self.AddMovementInput` (`KismetMathLibrary.GetForwardVector` (`KismetMathLibrary.MakeRotator` 0.0 0.0 _returnvalue_yaw_2)) ActionValue_Y)))

(event `self.ReceiveTick`
  (params (DeltaSeconds :type "Float (single-precision)"))
  (`self.ForwardLineTrace`))

(event `EnhancedInput|/Game/TrainGame/Core/Player/Input/IA_Look`
  (params (ActionValue :type "Vector2D Structure") (ElapsedSeconds :type "Float (double-precision)") (TriggeredSeconds :type "Float (double-precision)") (InputAction :type "InputAction Object Reference" :default "/Game/TrainGame/Core/Player/Input/IA_Look.IA_Look"))
  (:`Triggered`
    ;[1 1 1] L/R
    (`self.AddControllerYawInput` ActionValue_X)
    ;[1 1 1] U/D
    (`self.AddControllerPitchInput` ActionValue_Y)))

(event `EnhancedInput|/Game/TrainGame/Core/Player/Input/IA_Jump`
  (params (ActionValue :type Boolean) (ElapsedSeconds :type "Float (double-precision)") (TriggeredSeconds :type "Float (double-precision)") (InputAction :type "InputAction Object Reference" :default "/Game/TrainGame/Core/Player/Input/IA_Jump.IA_Jump"))
  (:`Triggered`
    (`self.Jump`))
  (:`Canceled`
    (`self.StopJumping`)))

(event `EnhancedInput|/Game/TrainGame/Core/Player/Input/IA_Grab`
  (params (ActionValue :type Boolean) (ElapsedSeconds :type "Float (double-precision)") (TriggeredSeconds :type "Float (double-precision)") (InputAction :type "InputAction Object Reference" :default "/Game/TrainGame/Core/Player/Input/IA_Grab.IA_Grab"))
  (:`Triggered`
    (`self.TrackBuild`)))

(fn `ForwardLineTrace`
  (bind _camera (`self.Camera`))
  (bind _returnvalue (`SceneComponent.K2_GetComponentLocation` _camera))
  (bind (_outhit _returnvalue_2) (`KismetSystemLibrary.LineTraceSingle` :`Start` _returnvalue :`End` (+ _returnvalue (* (`SceneComponent.GetForwardVector` _camera) (`self.CameraTraceLength`))) :`TraceChannel` "TraceTypeQuery1" :`DrawDebugType` "ForDuration"))
  (set `self.CameraTraceHitLocation` (`KismetMathLibrary.SelectVector` (`.Location` (`GameplayStatics.BreakHitResult` _outhit)) (`.TraceEnd` (`GameplayStatics.BreakHitResult` _outhit)) _returnvalue_2)))

(fn `HandleClick`)

(fn `SetupInputSystem`
  (bind _aspc_player_character (cast `/Game/TrainGame/Core/Player/PC_PlayerCharacter` (`self.GetController`)))
  (bind _returnvalue (pcsubsystem `EnhancedInputLocalPlayerSubsystem` _aspc_player_character))
  (`/Engine/EditorBlueprintResources/StandardMacros.IsValid` _returnvalue
    (:`Is Valid`
      (`EnhancedInputSubsystemInterface.AddMappingContext` _returnvalue "/Game/TrainGame/Core/Player/Input/IMC_Default.IMC_Default" 0 (struct)))))

(fn `TrackBuild`
  (bind _trackmanagerref (`self.TrackManagerRef`))
  (if (`self.IsBuilding?`)
    (`/Engine/EditorBlueprintResources/StandardMacros.IsValid` _trackmanagerref
      (:`Is Valid`
        (message `/Game/TrainGame/Core/Track/BPI_TrackInterface.RegisterTrackSegment` _trackmanagerref (`self.BuildingTrackSegmentRef`))
        (set `self.IsBuilding?` false)))
    (else
      (bind _returnvalue (`|SpawnActorFromClass` "/Game/TrainGame/Core/Track/BP_TrackSegment.BP_TrackSegment_C" (`KismetMathLibrary.MakeTransform` (+ (`self.CameraTraceHitLocation`) (0.0 0.0 10.0)) (`KismetMathLibrary.MakeRotator` 0.0 0.0 (`self.CurrentBuildRotation`))) "AlwaysSpawn" "MultiplyWithRoot" null null))
      (set `self.BuildingTrackSegmentRef` _returnvalue)
      (`KismetSystemLibrary.PrintString` "SpawnedTrack")
      (set `self.IsBuilding?` true))))

(fn `UserConstructionScript`)