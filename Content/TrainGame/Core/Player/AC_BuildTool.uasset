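; Player build-tool component for placing track segments and rolling stock via a spawned preview actor.
; Each update traces from the camera, snaps position and tangent to hit track segments, or uses scroll rotation off-track, then moves the preview.
; Track takes two clicks, anchoring the start then stretching End B; rolling stock takes one.
; Confirmed placements register with tag-located TrackManager or RollingStockManager, then a fresh GUID-named preview spawns.
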(event `self.ReceiveBeginPlay`
  (bind _asbp_character (cast `/Game/TrainGame/Core/Player/BP_Character` (`self.GetOwner`)))
  (set `self.CharacterRef` _asbp_character)
  (bind _outactors (`GameplayStatics.GetAllActorsWithTag` "TrackManager"))
  (bind _asbp_track_manager (cast `/Game/TrainGame/Core/Track/BP_TrackManager` (`|GetArrayItem` _outactors)))
  (set `self.TrackManagerRef` _asbp_track_manager)
  (bind _outactors_2 (`GameplayStatics.GetAllActorsWithTag` "RollingStockManager"))
  (bind _asbp_rolling_stock_manager (cast `/Game/TrainGame/Core/RollingStock/BP_RollingStockManager` (`|GetArrayItem` _outactors_2)))
  (set `self.RollingStockManagerRef` _asbp_rolling_stock_manager))

(fn `CheckForSnapToTrack`
  (bind _cameratracehitlocation (`self.CameraTraceHitLocation`))
  (set `self.IsSnapping?` false)
  (bind _asbp_track_segment (cast `/Game/TrainGame/Core/Track/BP_TrackSegment` (`self.CameraTraceHitActor`)) ; Just make sure it's a track segment. Otherwise, we try to send a message to things that don't implement the interface and it fails.
    (:`then`
      (bind (_snapsuccessful _snappedlocation _snappedtangent _snappedend _trackid) (message `/Game/TrainGame/Core/Track/BPI_TrackInterface.GetSnappedLocationAndTangent` _asbp_track_segment (select `/Game/TrainGame/Core/Player/E_BuildableType` (`self.CurrentBuildType`) :`NewEnumerator0` true) _cameratracehitlocation))
      (set `self.IsSnapping?` _snapsuccessful)
      (set `self.SnappedLocation` _snappedlocation)
      (bind _returnvalue (`KismetMathLibrary.SelectVector` _snappedtangent (`KismetMathLibrary.NegateVector` _snappedtangent) (`self.IsFirstClick?`)))
      (set `self.SnappedTangent` (select `/Game/TrainGame/Core/Track/Enum_TrackEnd` _snappedend :`NewEnumerator0` (`KismetMathLibrary.NegateVector` _returnvalue) :`NewEnumerator1` _returnvalue))
      (set `self.SnappedEnd` _snappedend)
      (set `self.SnappedTrackID` _trackid))
    (:`CastFailed`
      (set `self.SnappedLocation` _cameratracehitlocation)
      (set `self.SnappedTangent` (`KismetMathLibrary.GetForwardVector` (`KismetMathLibrary.MakeRotator` 0.0 0.0 (`self.ToolRotation`))))
      (set `self.SnappedTrackID` "None"))))

(fn `ClearBuildableActor`
  (bind _buildableactorref (`self.BuildableActorRef`))
  (`/Engine/EditorBlueprintResources/StandardMacros.IsValid` _buildableactorref
    (:`Is Valid`
      (`Actor.K2_DestroyActor` _buildableactorref)
      (set `self.BuildableActorRef` null))))

(fn `CreateBuildableActorFromType`
  (params (BuildableType :type "/Game/TrainGame/Core/Player/E_BuildableType Enum" :default "NewEnumerator0"))
  (bind _returnvalue (`KismetStringLibrary.Conv_StringToName` (`KismetGuidLibrary.Conv_GuidToString` (`KismetGuidLibrary.NewGuid`))))
  (bind _output_get (set `self.CurrentBuildType` BuildableType))
  (switch `/Game/TrainGame/Core/Player/E_BuildableType` _output_get
    (:`NewEnumerator0`
      (bind _returnvalue_2 (`|SpawnActorFromClass` "/Game/TrainGame/Core/Track/BP_TrackSegment.BP_TrackSegment_C" (`KismetMathLibrary.MakeTransform` (0.0 0.0 0.0)) "AlwaysSpawn" "MultiplyWithRoot" null _returnvalue null))
      (set `self.BuildableActorRef` _returnvalue_2))
    (:`NewEnumerator1`
      (bind _returnvalue_3 (`|SpawnActorFromClass` "/Game/TrainGame/Core/RollingStock/BP_RollingStock.BP_RollingStock_C" (`KismetMathLibrary.MakeTransform` (0.0 0.0 0.0)) "AlwaysSpawn" "MultiplyWithRoot" null _returnvalue null))
      (set `self.BuildableActorRef` _returnvalue_3))))

(fn `GetCameraTrace`
  (bind _characterref (`self.CharacterRef`))
  (`/Engine/EditorBlueprintResources/StandardMacros.IsValid` _characterref
    (:`Is Valid`
      (bind _tracehitresult (`/Game/TrainGame/Core/Player/BP_Character.CameraLineTrace` _characterref (`self.BuildableActorRef`) (`self.ToolTraceLength`)))
      (bind (_bblockinghit _binitialoverlap _time _distance _location _impactpoint _normal _impactnormal _physmat _hitactor _hitcomponent _hitbonename _bonename _hititem _elementindex _faceindex _tracestart _traceend) (`GameplayStatics.BreakHitResult` _tracehitresult))
      (set `self.CameraTraceHitLocation` (`KismetMathLibrary.SelectVector` _impactpoint _traceend _bblockinghit))
      (set `self.CameraTraceHitActor` _hitactor))))

(fn `HandleBuildTypeChanged`
  (params (NewBuildType :type "/Game/TrainGame/Core/Player/E_BuildableType Enum" :default "NewEnumerator0"))
  (if (`|EnumInequality` NewBuildType (`self.CurrentBuildType`))
    (`self.ClearBuildableActor`)
    (`self.CreateBuildableActorFromType` NewBuildType)))

(fn `HandlePrimaryClick`
  (bind _buildableactorref (`self.BuildableActorRef`))
  (switch `/Game/TrainGame/Core/Player/E_BuildableType` (`self.CurrentBuildType`)
    (:`NewEnumerator0`
      (if (`self.IsFirstClick?`)
        ;[1 1 1] "Set down" track, to start updating EndB
        (bind _asbp_track_segment (cast `/Game/TrainGame/Core/Track/BP_TrackSegment` (`self.BuildableActorRef`)))
        (`Actor.K2_SetActorLocationAndRotation` :`self` _asbp_track_segment :`NewLocation` (`self.SnappedLocation`))
        (`SplineComponent.SetTangentAtSplinePoint` (`/Game/TrainGame/Core/Track/BP_TrackSegment.Spline` _asbp_track_segment) 0 (`self.SnappedTangent`) "Local" true)
        (set `self.IsFirstClick?` false)
        (else
          ;[1 1 1] Register Then Reset Build Actor
          (bind _asbp_track_segment_2 (cast `/Game/TrainGame/Core/Track/BP_TrackSegment` _buildableactorref))
          (message `/Game/TrainGame/Core/Track/BPI_TrackManagerInterface.RegisterTrackSegment` (`self.TrackManagerRef`) _asbp_track_segment_2)
          (`self.OnToolEnter` :!label _label)
          (set `self.IsFirstClick?` true))))
    (:`NewEnumerator1`
      (bind _asbp_rolling_stock (cast `/Game/TrainGame/Core/RollingStock/BP_RollingStock` _buildableactorref))
      (message `/Game/TrainGame/Core/RollingStock/BPI_RollingStockManager.RegisterRollingStock` (`self.RollingStockManagerRef`) _asbp_rolling_stock)
      (goto _label))))

(fn `HandleScroll`
  (params (Delta :type "Float (double-precision)"))
  (set `self.ToolRotation` (`KismetMathLibrary.FWrap` (+ (`self.ToolRotation`) (* Delta 11.25)) -180.0 180.0)))

(fn `HandleSecondaryClick`
  (if (`self.IsFirstClick?`)
    _))

(fn `OnToolEnter`
  (`self.CreateBuildableActorFromType` (`self.CurrentBuildType`)))

(fn `OnToolExit`
  (`self.ClearBuildableActor`)
  (set `self.IsFirstClick?` true))

(fn `Update`
  (bind _buildableactorref (`self.BuildableActorRef`))
  (`self.GetCameraTrace`)
  (`self.CheckForSnapToTrack`)
  (switch `/Game/TrainGame/Core/Player/E_BuildableType` (`self.CurrentBuildType`)
    (:`NewEnumerator0`
      (set `self.SnappedLocation` (+ (`self.SnappedLocation`) (0.0 0.0 10.0)))
      (if (`self.IsFirstClick?`)
        (`/Engine/EditorBlueprintResources/StandardMacros.IsValid` _buildableactorref :!label _label
          (:`Is Valid`
            (`Actor.K2_SetActorLocationAndRotation` _buildableactorref (`self.SnappedLocation`) (`KismetMathLibrary.Conv_VectorToRotator` (`self.SnappedTangent`)) false false)))
        (else
          (bind _asbp_track_segment (cast `/Game/TrainGame/Core/Track/BP_TrackSegment` _buildableactorref))
          (`/Game/TrainGame/Core/Track/BP_TrackSegment.Set End B Location And Tangent` _asbp_track_segment (`self.SnappedLocation`) (`self.SnappedTangent`)))))
    (:`NewEnumerator1`
      (goto _label))))