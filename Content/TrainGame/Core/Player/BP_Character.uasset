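; Player character for a train game, handling Enhanced Input setup, movement, look and jump.
; Tick, clicks, scroll and build-type changes forward to the ACBuildTool component.
; Its own build functions, which the event graph never calls, spawn GUID-tagged track segments or rolling stock, position them at a camera trace hit, and register them with tag-found managers.
; Those functions snap pieces to spline endpoints with matched tangents, or anywhere along the spline.
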(event `self.ReceiveBeginPlay`
  (`|ExecutionSequence`
    (:`then_0`
      (`self.SetupInputSystem`))
    (:`then_1`
      (bind _aspc_player (cast `/Game/TrainGame/Core/Player/PC_Player` (`self.GetController`)))
      (set `self.PlayerControllerRef` _aspc_player))
    (:`then_2`
      (bind _outactors (`GameplayStatics.GetAllActorsWithTag` "TrackManager"))
      (bind _output (`|GetArrayItem` _outactors))
      (cast `/Game/TrainGame/Core/Track/BP_TrackManager` _output)
      (set `self.TrackManagerRef` _output)
      (bind _outactors_2 (`GameplayStatics.GetAllActorsWithTag` "RollingStockManager"))
      (bind _output_2 (`|GetArrayItem` _outactors_2))
      (cast `/Game/TrainGame/Core/RollingStock/BP_RollingStockManager` _output_2)
      (set `self.RollingStockManagerRef` _output_2))))

(event `self.ReceiveTick`
  (params (DeltaSeconds :type "Float (single-precision)"))
  (`/Game/TrainGame/Core/Player/AC_BuildTool.Update` (`self.AC_BuildTool`)))

(event `/Game/TrainGame/Core/Player/BPI_PlayerPawn.HandleMove`
  (params (Axis :type "Vector2D Structure"))
  (bind (_returnvalue_roll _returnvalue_pitch _returnvalue_yaw) (`KismetMathLibrary.BreakRotator` (`self.GetControlRotation`)))
  (bind (_x _y) (`KismetMathLibrary.BreakVector2D` Axis))
  (bind (_returnvalue_roll_2 _returnvalue_pitch_2 _returnvalue_yaw_2) (`KismetMathLibrary.BreakRotator` (`self.GetControlRotation`)))
  ;[1 1 1] Movement Control Logic
  (`self.AddMovementInput` (`KismetMathLibrary.GetRightVector` (`KismetMathLibrary.MakeRotator` _returnvalue_roll 0.0 _returnvalue_yaw)) _x)
  (`self.AddMovementInput` (`KismetMathLibrary.GetForwardVector` (`KismetMathLibrary.MakeRotator` 0.0 0.0 _returnvalue_yaw_2)) _y))

(event `/Game/TrainGame/Core/Player/BPI_PlayerPawn.HandleLook`
  (params (Axis :type "Vector2D Structure"))
  (bind (_x _y) (`KismetMathLibrary.BreakVector2D` Axis))
  ;[1 1 1] Movement Control Logic
  ;;[1 1 1] L/R
  (`self.AddControllerYawInput` _x)
  ;;[1 1 1] U/D
  (`self.AddControllerPitchInput` _y))

(event `/Game/TrainGame/Core/Player/BPI_PlayerPawn.OnJumpPressed`
  ;[1 1 1] Movement Control Logic
  (`self.Jump`))

(event `/Game/TrainGame/Core/Player/BPI_PlayerPawn.OnJumpReleased`
  ;[1 1 1] Movement Control Logic
  (`self.StopJumping`))

(event `/Game/TrainGame/Core/Player/BPI_BuildTool.EnterTool`
  ;[1 1 1] Build Control Logic
  (`/Game/TrainGame/Core/Player/AC_BuildTool.OnToolEnter` (`self.AC_BuildTool`)))

(event `/Game/TrainGame/Core/Player/BPI_BuildTool.ExitTool`
  ;[1 1 1] Build Control Logic
  (`/Game/TrainGame/Core/Player/AC_BuildTool.OnToolExit` (`self.AC_BuildTool`)))

(event `/Game/TrainGame/Core/Player/BPI_BuildTool.HandlePrimaryClick`
  ;[1 1 1] Build Control Logic
  (`/Game/TrainGame/Core/Player/AC_BuildTool.HandlePrimaryClick` (`self.AC_BuildTool`)))

(event `/Game/TrainGame/Core/Player/BPI_BuildTool.HandleSecondaryClick`
  ;[1 1 1] Build Control Logic
  (`/Game/TrainGame/Core/Player/AC_BuildTool.HandleSecondaryClick` (`self.AC_BuildTool`)))

(event `/Game/TrainGame/Core/Player/BPI_BuildTool.HandleScroll`
  (params (Delta :type "Float (double-precision)"))
  ;[1 1 1] Build Control Logic
  (`/Game/TrainGame/Core/Player/AC_BuildTool.HandleScroll` (`self.AC_BuildTool`) Delta))

(event `/Game/TrainGame/Core/Player/BPI_BuildTool.OnBuildTypeChanged`
  (params (NewBuildType :type "/Game/TrainGame/Core/Player/E_BuildableType Enum" :default "NewEnumerator0"))
  ;[1 1 1] Build Control Logic
  (`/Game/TrainGame/Core/Player/AC_BuildTool.HandleBuildTypeChanged` (`self.AC_BuildTool`) NewBuildType))

(event `/Game/TrainGame/Core/Player/BPI_PlayerPawn.HandleInteractionModeChanged`
  (params (NewMode :type "/Game/TrainGame/Core/Player/E_InteractionMode Enum" :default "NewEnumerator0"))
  (`self.Update Interaction Mode Changed` NewMode))

(fn `ApplyBuildPiece`
  (switch `/Game/TrainGame/Core/Player/E_BuildableType` (`self.CurrentBuildableType`)
    (:`NewEnumerator0`
      (`self.Place Track End`))
    (:`NewEnumerator1`
      (`self.PlaceRollingStock`))))

(fn `ApplyBuildPieceRotationDelta`
  (params (Delta :type "Float (double-precision)"))
  (set `self.CurrentBuildRotation` (`KismetMathLibrary.FWrap` (+ (`self.CurrentBuildRotation`) (* Delta 11.25)) -180.0 180.0)))

(fn `CameraLineTrace`
  (params (IgnoreActor :type "Actor Object Reference") (TraceLength :type "Float (double-precision)"))
  (returns (TraceHitResult :type "HitResult Structure"))
  (bind _camera (`self.Camera`))
  (bind _returnvalue (`SceneComponent.K2_GetComponentLocation` _camera))
  (bind _outhit (`KismetSystemLibrary.SphereTraceSingle` _returnvalue (+ _returnvalue (* (`SceneComponent.GetForwardVector` _camera) TraceLength)) 10.0 "TraceTypeQuery1" false (`|MakeArray` IgnoreActor)))
  (return _outhit))

(fn `CheckForIntersect`
  (bind _asbp_track_segment (cast `/Game/TrainGame/Core/Track/BP_TrackSegment` (`self.CameraTraceHitActor`)))
  (if (not (`self.isSnapping?`))
    (set `self.isSnapping?` true)
    (bind _spline (`/Game/TrainGame/Core/Track/BP_TrackSegment.Spline` _asbp_track_segment))
    (bind _returnvalue (`SplineComponent.GetDistanceAlongSplineAtLocation` _spline (`self.CameraTraceHitLocation`) "World"))
    (set `self.SnappedLocation` (`SplineComponent.GetLocationAtDistanceAlongSpline` _spline _returnvalue "World"))
    (set `self.SnappedTangent` (`SplineComponent.GetTangentAtDistanceAlongSpline` _spline _returnvalue "World"))))

(fn `CheckForSnap`
  (locals (SnappingDistance :type "Float (double-precision)" :default 100.0))
  (bind _cameratracehitlocation (`self.CameraTraceHitLocation`))
  (bind _snappingdistance (`local.SnappingDistance`))
  (set `self.isSnapping?` false)
  (bind _asbp_track_segment (cast `/Game/TrainGame/Core/Track/BP_TrackSegment` (`self.CameraTraceHitActor`)))
  (if true
    (bind _spline (`/Game/TrainGame/Core/Track/BP_TrackSegment.Spline` _asbp_track_segment))
    (bind _returnvalue (`SplineComponent.GetLocationAtSplinePoint` _spline 0 "World"))
    (if (> (`KismetMathLibrary.Vector_Distance` _cameratracehitlocation _returnvalue) _snappingdistance)
      (bind _returnvalue_2 (`SplineComponent.GetLocationAtSplinePoint` _spline 1 "World"))
      (if (not (> (`KismetMathLibrary.Vector_Distance` _cameratracehitlocation _returnvalue_2) _snappingdistance))
        (set `self.isSnapping?` true)
        (set `self.SnappedLocation` _returnvalue_2)
        (set `self.SnappedTangent` (`KismetMathLibrary.Normal` (`SplineComponent.GetTangentAtSplinePoint` _spline 1 "World")))
        (set `self.SnappedEnd` "NewEnumerator1")
        (bind _trackid (`/Game/TrainGame/Core/Track/BP_TrackSegment.TrackID` _asbp_track_segment))
        (set `self.SnappedTrackID` _trackid))
      (else
        (set `self.isSnapping?` true)
        (set `self.SnappedLocation` _returnvalue)
        (set `self.SnappedTangent` (`KismetMathLibrary.Normal` (`SplineComponent.GetTangentAtSplinePoint` _spline 0 "World")))
        (set `self.SnappedEnd` "NewEnumerator0")
        (set `self.SnappedTrackID` _trackid)))))

(fn `ClearBuildPiece`
  (bind _buildingtracksegmentref (`self.BuildingTrackSegmentRef`))
  (`/Engine/EditorBlueprintResources/StandardMacros.IsValid` _buildingtracksegmentref
    (:`Is Valid`
      (`self.K2_DestroyActor` _buildingtracksegmentref)
      (set `self.BuildingTrackSegmentRef` null))))

(fn `GetSnap`
  (params (TrackEnd :type "/Game/TrainGame/Core/Track/Enum_TrackEnd Enum" :default "NewEnumerator0"))
  (returns (Location :type "Vector Structure") (Tangent :type "Vector Structure") (TrackID :type Name))
  (bind _issnapping_ (`self.isSnapping?`))
  (bind _snappedtangent (`self.SnappedTangent`))
  (bind _returnvalue (select `/Game/TrainGame/Core/Track/Enum_TrackEnd` TrackEnd :`NewEnumerator0` _snappedtangent :`NewEnumerator1` (`KismetMathLibrary.NegateVector` _snappedtangent)))
  (return (`KismetMathLibrary.SelectVector` (`self.SnappedLocation`) (+ (`self.CameraTraceHitLocation`) (0.0 0.0 10.0)) _issnapping_) (`KismetMathLibrary.SelectVector` (select `/Game/TrainGame/Core/Track/Enum_TrackEnd` (`self.SnappedEnd`) :`NewEnumerator0` (`KismetMathLibrary.NegateVector` _returnvalue) :`NewEnumerator1` _returnvalue) (`KismetMathLibrary.GetForwardVector` (`KismetMathLibrary.MakeRotator` 0.0 0.0 (`self.CurrentBuildRotation`))) _issnapping_) (`KismetMathLibrary.SelectName` (`self.SnappedTrackID`) "None" _issnapping_)))

(fn `HandleClick`)

(fn `Place Track End`
  (bind _trackmanagerref (`self.TrackManagerRef`))
  (bind _buildingtracksegmentref (`self.BuildingTrackSegmentRef`))
  (if (`self.isBuilding?`)
    (`/Engine/EditorBlueprintResources/StandardMacros.IsValid` _trackmanagerref
      (:`Is Valid`
        (message `/Game/TrainGame/Core/Track/BPI_TrackManagerInterface.RegisterTrackSegment` _trackmanagerref (`self.BuildingTrackSegmentRef`))
        (`self.SetupBuildPiece`)
        (`KismetSystemLibrary.PrintString` "Placed Track End B")
        (set `self.isBuilding?` false)))
    (else
      (`/Engine/EditorBlueprintResources/StandardMacros.IsValid` _buildingtracksegmentref
        (:`Is Valid`
          (bind (_location _tangent) (`self.GetSnap` "NewEnumerator0"))
          (`self.K2_SetActorLocationAndRotation` :`self` _buildingtracksegmentref :`NewLocation` _location)
          (`SplineComponent.SetTangentAtSplinePoint` (`/Game/TrainGame/Core/Track/BP_TrackSegment.Spline` _buildingtracksegmentref) 0 _tangent "Local" true)
          (`KismetSystemLibrary.PrintString` "Placed Track End A")
          (set `self.isBuilding?` true))))))

(fn `PlaceRollingStock`
  (bind _buildingrollingstockref (`self.BuildingRollingStockRef`))
  (bind _rollingstockmanagerref (`self.RollingStockManagerRef`))
  (`/Engine/EditorBlueprintResources/StandardMacros.IsValid` _rollingstockmanagerref
    (:`Is Valid`
      (message `/Game/TrainGame/Core/RollingStock/BPI_RollingStockManager.RegisterRollingStock` _rollingstockmanagerref _buildingrollingstockref)
      (`/Game/TrainGame/Core/RollingStock/BP_RollingStock.EnablePlayerCollision` _buildingrollingstockref)
      (`self.SetupBuildPiece`)
      (`KismetSystemLibrary.PrintString` "Placed Rolling Stock")
      (set `self.isBuilding?` false))))

(fn `PrintDebugInfo`
  (`KismetSystemLibrary.PrintString` (`KismetTextLibrary.Conv_TextToString` (`|FormatText` "Build Mode Active: {bool}" (`self.isBuildModeActive?`))) true true (struct :`G` 0.66 :`B` 1.0 :`A` 1.0) 2.0 "BuildModeActive")
  (`KismetSystemLibrary.PrintString` (`KismetTextLibrary.Conv_TextToString` (`|FormatText` "Current Build Rotation: {rot}" (`self.CurrentBuildRotation`))) true true (struct :`G` 0.66 :`B` 1.0 :`A` 1.0) 2.0 "CurrentBuildRot")
  (`KismetSystemLibrary.PrintString` (`KismetMathLibrary.SelectString` "Updating Build Piece End" (`KismetMathLibrary.SelectString` "Updating Build Piece" "Not Building" (`self.isBuildModeActive?`)) (`self.isBuilding?`)) true true (struct :`R` 0.331464 :`G` 1.0 :`B` 0.057331 :`A` 1.0) 2.0 "UpdateingBuildPiece"))

(fn `SetupBuildPiece`
  (bind _returnvalue (`KismetStringLibrary.Conv_StringToName` (`KismetSystemLibrary.MakeLiteralString` (`KismetGuidLibrary.Conv_GuidToString` (`KismetGuidLibrary.NewGuid`)))))
  (switch `/Game/TrainGame/Core/Player/E_BuildableType` (`self.CurrentBuildableType`)
    (:`NewEnumerator0`
      (bind _returnvalue_2 (`|SpawnActorFromClass` "/Game/TrainGame/Core/Track/BP_TrackSegment.BP_TrackSegment_C" (`KismetMathLibrary.MakeTransform` (0.0 0.0 0.0)) "AlwaysSpawn" "MultiplyWithRoot" null _returnvalue null))
      (set `self.BuildingTrackSegmentRef` _returnvalue_2))
    (:`NewEnumerator1`
      (bind _returnvalue_3 (`|SpawnActorFromClass` "/Game/TrainGame/Core/RollingStock/BP_RollingStock.BP_RollingStock_C" (`KismetMathLibrary.MakeTransform` (0.0 0.0 0.0)) "AlwaysSpawn" "MultiplyWithRoot" null _returnvalue null))
      (set `self.BuildingRollingStockRef` _returnvalue_3))))

(fn `SetupInputSystem`
  (bind _aspc_player (cast `/Game/TrainGame/Core/Player/PC_Player` (`self.GetController`)))
  (bind _returnvalue (pcsubsystem `EnhancedInputLocalPlayerSubsystem` _aspc_player))
  (`/Engine/EditorBlueprintResources/StandardMacros.IsValid` _returnvalue
    (:`Is Valid`
      (`EnhancedInputSubsystemInterface.AddMappingContext` _returnvalue "/Game/TrainGame/Core/Player/Input/IMC_Default.IMC_Default" 0 (struct)))))

(fn `Update Interaction Mode Changed`
  (params (NewInteractionMode :type "/Game/TrainGame/Core/Player/E_InteractionMode Enum" :default "NewEnumerator0"))
  (set `self.CurrentInteractionMode` NewInteractionMode))

(fn `UpdateBuildableTypeChanged`
  (params (CurrentBuildableType :type "/Game/TrainGame/Core/Player/E_BuildableType Enum" :default "NewEnumerator0"))
  (set `self.CurrentBuildableType` CurrentBuildableType)
  (`self.SetupBuildPiece`))

(fn `UpdateBuildPiece`
  (bind _buildingtracksegmentref (`self.BuildingTrackSegmentRef`))
  (bind _buildingtracksegmentref_2 (`self.BuildingTrackSegmentRef`))
  (bind _buildingrollingstockref (`self.BuildingRollingStockRef`))
  (switch `/Game/TrainGame/Core/Player/E_BuildableType` (`self.CurrentBuildableType`)
    (:`NewEnumerator0`
      ;[1 1 1] Track Segment
      (if (`self.isBuilding?`)
        ;;[1 1 1] End A
        (`/Engine/EditorBlueprintResources/StandardMacros.IsValid` _buildingtracksegmentref
          (:`Is Valid`
            (`self.CheckForSnap`)
            (`self.CheckForIntersect`)
            (bind (_location _tangent) (`self.GetSnap` "NewEnumerator1"))
            (`/Game/TrainGame/Core/Track/BP_TrackSegment.Set End B Location And Tangent` _buildingtracksegmentref _location _tangent)
            (setmembers `/Game/TrainGame/Core/Track/Struct_TrackConnection` :`StructRef` (`/Game/TrainGame/Core/Track/BP_TrackSegment.EndA` _buildingtracksegmentref) :`ConnectedTrackID` "None")))
        (else
          ;;[1 1 1] End B
          (`/Engine/EditorBlueprintResources/StandardMacros.IsValid` _buildingtracksegmentref_2
            (:`Is Valid`
              (`self.CheckForSnap`)
              (`self.CheckForIntersect`)
              (bind (_location_2 _tangent_2) (`self.GetSnap` "NewEnumerator0"))
              (`self.K2_SetActorLocationAndRotation` _buildingtracksegmentref_2 _location_2 (`KismetMathLibrary.Conv_VectorToRotator` _tangent_2) false false))))))
    (:`NewEnumerator1`
      ;[1 1 1] Rolling Stock
      (`/Engine/EditorBlueprintResources/StandardMacros.IsValid` _buildingrollingstockref
        (:`Is Valid`
          (`self.CheckForSnap`)
          (`self.CheckForIntersect`)
          (bind (_location_3 _tangent_3) (`self.GetSnap` "NewEnumerator1"))
          (`self.K2_SetActorLocationAndRotation` _buildingrollingstockref _location_3 (`KismetMathLibrary.Conv_VectorToRotator` _tangent_3) false false))))))

(fn `UpdateDebugArrow`
  (bind _arrowref (`self.ArrowRef`))
  (`/Engine/EditorBlueprintResources/StandardMacros.IsValid` _arrowref
    (:`Is Valid`
      (`self.K2_SetActorLocationAndRotation` _arrowref (`self.CameraTraceHitLocation`) (`KismetMathLibrary.Conv_VectorToRotator` (`KismetMathLibrary.GetForwardVector` (`KismetMathLibrary.MakeRotator` 0.0 0.0 (`self.CurrentBuildRotation`)))) false false))))

(fn `UserConstructionScript`)