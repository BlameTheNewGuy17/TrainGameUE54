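; Player controller for TrainGame that creates the HUD and menu widgets and routes player input to the possessed pawn.
; Enhanced Input move, look, jump, click and scroll events pass a menu-open macro gate, then reach the pawn as messages, keeping the controller decoupled.
; P toggles the menu and input mode; B toggles build mode, which enables placing and rotating buildables.
; Interaction mode changes propagate to both pawn and HUD.
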(event `self.ReceiveBeginPlay`
  (bind _asgi_core (cast `/Game/TrainGame/Core/GI_Core` (`GameplayStatics.GetGameInstance`)))
  (set `self.Game Instance Ref` _asgi_core)
  (bind _returnvalue (`|CreateWidget` "/Game/TrainGame/Core/UI/WBP_Menu.WBP_Menu_C"))
  (set `self.MenuWidgetRef` _returnvalue)
  (bind _returnvalue_2 (`|CreateWidget` "/Game/TrainGame/Core/Player/WBP_HUD.WBP_HUD_C"))
  (bind _output_get (set `self.HUDWidgetRef` _returnvalue_2))
  (`UserWidget.AddToViewport` _output_get 0)
  (set `self.InteractionMode` "NewEnumerator0"))

(event `self.ReceivePossess`
  (params (PossessedPawn :type "Pawn Object Reference"))
  (bind _output_get (set `self.Possessed Pawn` PossessedPawn))
  (message `/Game/TrainGame/Core/Player/BPI_PlayerPawn.OnInteractionModeChanged` _output_get "NewEnumerator0"))

(event `EnhancedInput|/Game/TrainGame/Core/Player/Input/IA_Move`
  (params (ActionValue :type "Vector2D Structure") (ElapsedSeconds :type "Float (double-precision)") (TriggeredSeconds :type "Float (double-precision)") (InputAction :type "InputAction Object Reference" :default "/Game/TrainGame/Core/Player/Input/IA_Move.IA_Move"))
  (:`Triggered`
    (`self.CheckMenuOpen`
      (:`false`
        (message `/Game/TrainGame/Core/Player/BPI_PlayerPawn.HandleMove` (`self.Possessed Pawn`) (`KismetMathLibrary.MakeVector2D` ActionValue_X ActionValue_Y))))))

(event `EnhancedInput|/Game/TrainGame/Core/Player/Input/IA_Look`
  (params (ActionValue :type "Vector2D Structure") (ElapsedSeconds :type "Float (double-precision)") (TriggeredSeconds :type "Float (double-precision)") (InputAction :type "InputAction Object Reference" :default "/Game/TrainGame/Core/Player/Input/IA_Look.IA_Look"))
  (:`Triggered`
    (`self.CheckMenuOpen`
      (:`false`
        (message `/Game/TrainGame/Core/Player/BPI_PlayerPawn.HandleLook` (`self.Possessed Pawn`) (`KismetMathLibrary.MakeVector2D` ActionValue_X ActionValue_Y))))))

(event `EnhancedInput|/Game/TrainGame/Core/Player/Input/IA_Jump`
  (params (ActionValue :type Boolean) (ElapsedSeconds :type "Float (double-precision)") (TriggeredSeconds :type "Float (double-precision)") (InputAction :type "InputAction Object Reference" :default "/Game/TrainGame/Core/Player/Input/IA_Jump.IA_Jump"))
  (bind _possessed_pawn (`self.Possessed Pawn`))
  (:`Triggered`
    (`self.CheckMenuOpen`
      (:`false`
        (message `/Game/TrainGame/Core/Player/BPI_PlayerPawn.OnJumpPressed` _possessed_pawn))))
  (:`Canceled`
    (`self.CheckMenuOpen`
      (:`false`
        (message `/Game/TrainGame/Core/Player/BPI_PlayerPawn.OnJumpReleased` _possessed_pawn)))))

(event `EnhancedInput|/Game/TrainGame/Core/Player/Input/IA_Click`
  (params (ActionValue :type Boolean) (ElapsedSeconds :type "Float (double-precision)") (TriggeredSeconds :type "Float (double-precision)") (InputAction :type "InputAction Object Reference" :default "/Game/TrainGame/Core/Player/Input/IA_Click.IA_Click"))
  (:`Triggered`
    (switch `/Game/TrainGame/Core/Player/E_InteractionMode` (`self.InteractionMode`)
      (:`NewEnumerator1`
        (`self.CheckMenuOpen`
          (:`false`
            (message `/Game/TrainGame/Core/Player/BPI_PlayerPawn.OnPlaceBuildable` (`self.Possessed Pawn`) 0)))))))

(event `EnhancedInput|/Game/TrainGame/Core/Player/Input/IA_Scroll`
  (params (ActionValue :type "Float (double-precision)") (ElapsedSeconds :type "Float (double-precision)") (TriggeredSeconds :type "Float (double-precision)") (InputAction :type "InputAction Object Reference" :default "/Game/TrainGame/Core/Player/Input/IA_Scroll.IA_Scroll"))
  (:`Triggered`
    (switch `/Game/TrainGame/Core/Player/E_InteractionMode` (`self.InteractionMode`)
      (:`NewEnumerator1`
        (`self.CheckMenuOpen`
          (:`false`
            (message `/Game/TrainGame/Core/Player/BPI_PlayerPawn.HandleRotateBuild` (`self.Possessed Pawn`) ActionValue)))))))

(event `Key|P`
  (params (Key :type "Key Structure"))
  (:`Pressed`
    (`/Engine/EditorBlueprintResources/StandardMacros.IsValid` (`self.MenuWidgetRef`)
      (:`Is Valid`
        (`self.Toggle Menu Visibility` false)))))

(event `Key|B`
  (params (Key :type "Key Structure"))
  (:`Pressed`
    (switch `/Game/TrainGame/Core/Player/E_InteractionMode` (`self.InteractionMode`)
      (:`NewEnumerator0`
        (`self.SetInteractionMode` "NewEnumerator1" :!label _label))
      (:`NewEnumerator1`
        (`self.SetInteractionMode` "NewEnumerator0"))
      (:`NewEnumerator2`
        (goto _label)))))

(fn `SetInteractionMode`
  (params (NewMode :type "/Game/TrainGame/Core/Player/E_InteractionMode Enum" :default "NewEnumerator0"))
  (bind _hudwidgetref (`self.HUDWidgetRef`))
  (bind _output_get (set `self.InteractionMode` NewMode))
  (message `/Game/TrainGame/Core/Player/BPI_PlayerPawn.OnInteractionModeChanged` (`self.Possessed Pawn`) _output_get)
  (`/Engine/EditorBlueprintResources/StandardMacros.IsValid` _hudwidgetref
    (:`Is Valid`
      (set `/Game/TrainGame/Core/Player/WBP_HUD.CurrentInteractionMode` _output_get _hudwidgetref))))

(fn `Toggle Menu Visibility`
  (params (`Show Mouse Cursor` :type Boolean))
  (returns (`MenuOpen?` :type Boolean))
  (bind _menuwidgetref (`self.MenuWidgetRef`))
  (bind _bismenuopen (`self.bIsMenuOpen`))
  (`/Engine/EditorBlueprintResources/StandardMacros.IsValid` _menuwidgetref
    (:`Is Valid`
      (if (`self.bIsMenuOpen`)
        (`Widget.RemoveFromParent` _menuwidgetref)
        (`WidgetBlueprintLibrary.SetInputMode_GameOnly` self)
        (set `self.bIsMenuOpen` false)
        (`WidgetBlueprintLibrary.SetFocusToGameViewport`)
        (else
          (`UserWidget.AddToViewport` _menuwidgetref 0)
          (`WidgetBlueprintLibrary.SetInputMode_GameAndUIEx` self _menuwidgetref "LockAlways" false)
          (set `self.bIsMenuOpen` true)))
      (set `self.bShowMouseCursor` _bismenuopen)
      (return _bismenuopen))))

(fn `UserConstructionScript`)