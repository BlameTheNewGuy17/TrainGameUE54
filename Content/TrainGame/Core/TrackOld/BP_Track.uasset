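; Train track actor that builds two rails and evenly spaced ties along a spline when GenerateRailsAndTies is called.
; GenerateTrack scales each spline tangent to spline length, then rebuilds rails as short spline-mesh segments offset by half the gauge, with length-normalized tangents.
; Ties are instanced static meshes placed and rotated along the spline.
; Straight and arc spline-shaping helpers exist, but the construction script's curve and generation calls are disconnected.
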(event `GenerateRailsAndTies`
  (`self.GenerateTrack`))

(fn `AssignSplineCurves`
  (`self.SetSplineCurve` (`self.Spline`) (`self.Length`)))

(fn `GenerateRailMesh`
  (params (SplineRef :type "SplineComponent Object Reference") (SplineDistanceStart :type "Float (single-precision)") (SplineDistanceEnd :type "Float (double-precision)") (RailGaugeOffset :type "Float (double-precision)"))
  (bind _returnvalue (- SplineDistanceEnd SplineDistanceStart))
  (bind _returnvalue_2 (`AddComponent|NODE_AddSplineMeshComponent-0` :`bManualAttachment` true))
  (`KismetArrayLibrary.Array_Add` (`self.RailMeshRefs`) _returnvalue_2)
  (`SplineMeshComponent.SetStartAndEnd` _returnvalue_2 (+ (+ (`SplineComponent.GetLocationAtDistanceAlongSpline` SplineRef SplineDistanceStart "World") (* (`SplineComponent.GetRightVectorAtDistanceAlongSpline` SplineRef SplineDistanceStart "Local") RailGaugeOffset)) (`KismetMathLibrary.MakeVector` 0.0 0.0 (`self.HeightOffset`))) (* (`KismetMathLibrary.Normal` (`SplineComponent.GetTangentAtDistanceAlongSpline` SplineRef SplineDistanceStart "World")) _returnvalue) (+ (+ (`SplineComponent.GetLocationAtDistanceAlongSpline` SplineRef SplineDistanceEnd "World") (* (`SplineComponent.GetRightVectorAtDistanceAlongSpline` SplineRef SplineDistanceEnd "Local") RailGaugeOffset)) (`KismetMathLibrary.MakeVector` 0.0 0.0 (`self.HeightOffset`))) (* (`KismetMathLibrary.Normal` (`SplineComponent.GetTangentAtDistanceAlongSpline` SplineRef SplineDistanceEnd "World")) _returnvalue) true))

(fn `GenerateRails`
  (bind _railmeshlength (`self.RailMeshLength`))
  (bind _spline (`self.Spline`))
  (bind _returnvalue (/ (`self.RailGauge`) 2.0))
  (`/Game/TrainGame/Core/ProcFuncs.Delete and Clear Actor Component Array` (`self.RailMeshRefs`))
  (for _index (range (+ (`KismetMathLibrary.FFloor` (/ (`SplineComponent.GetSplineLength` (`self.Spline`)) (`self.RailMeshLength`))) 1))
    (bind _returnvalue_2 (* _index _railmeshlength))
    (bind _returnvalue_3 (+ _returnvalue_2 _railmeshlength))
    (`self.GenerateRailMesh` _spline _returnvalue_2 _returnvalue_3 _returnvalue) ; Right Rail
    (`self.GenerateRailMesh` _spline _returnvalue_2 _returnvalue_3 (* _returnvalue -1.0)) ; Left Rail
  ))

(fn `GenerateTies`
  (bind _spline (`self.Spline`))
  (bind _tieseparation (`self.TieSeparation`))
  (`InstancedStaticMeshComponent.ClearInstances` (`self.InstancedStaticMesh`))
  (for _index (range (`KismetMathLibrary.FFloor` (/ (`SplineComponent.GetSplineLength` (`self.Spline`)) (`self.TieSeparation`))))
    (bind _returnvalue (+ (* _index _tieseparation) (/ _tieseparation 2.0)))
    (`InstancedStaticMeshComponent.AddInstance` (`self.InstancedStaticMesh`) (`KismetMathLibrary.MakeTransform` (+ (`SplineComponent.GetLocationAtDistanceAlongSpline` _spline _returnvalue "Local") (`KismetMathLibrary.MakeVector` 0.0 0.0 (`self.HeightOffset`))) (`SplineComponent.GetRotationAtDistanceAlongSpline` _spline _returnvalue "Local")) false)))

(fn `GenerateTrack`
  (`self.SetSplineTangents`)
  (`self.GenerateRails`)
  (`self.GenerateTies`))

(fn `SetSplineCurve`
  (params (SplineRef :type "SplineComponent Object Reference") (Length :type "Float (double-precision)" :default 100.0) (CurveDegrees :type "Float (double-precision)"))
  (bind _returnvalue (`self.GetActorForwardVector`))
  (bind _returnvalue_2 (* (`self.ArcTangentMultiplier`) 0.75))
  (`SplineComponent.SetTangentAtSplinePoint` SplineRef 0 (* (* (`self.GetActorForwardVector`) Length) _returnvalue_2) "Local" false)
  (`SplineComponent.SetLocationAtSplinePoint` SplineRef 1 (* Length (`KismetMathLibrary.RotateAngleAxis` _returnvalue (/ CurveDegrees 2.0) (0.0 0.0 1.0))) "Local" false)
  (`SplineComponent.SetTangentAtSplinePoint` SplineRef 1 (* (* Length (`KismetMathLibrary.RotateAngleAxis` _returnvalue CurveDegrees (0.0 0.0 1.0))) _returnvalue_2) "Local" true))

(fn `SetSplinePointTangentLength`
  (params (SplinePoint :type Integer))
  (bind _spline (`self.Spline`))
  ;[1 1 1] Set the tangent to be the same as the spline length
  (`SplineComponent.SetTangentAtSplinePoint` _spline SplinePoint (* (`SplineComponent.GetSplineLength` _spline) (`KismetMathLibrary.Normal` (`SplineComponent.GetTangentAtSplinePoint` _spline SplinePoint "Local"))) "Local" true))

(fn `SetSplineStraight`
  (bind _spline (`self.Spline`))
  (bind _returnvalue (* (`SceneComponent.GetForwardVector` _spline) (`self.Length`)))
  (`SplineComponent.SetLocationAtSplinePoint` _spline 1 (+ (`SplineComponent.GetLocationAtSplinePoint` _spline 0 "Local") _returnvalue) "Local" false)
  (`SplineComponent.SetTangentAtSplinePoint` _spline 0 _returnvalue "Local" false)
  (`SplineComponent.SetTangentAtSplinePoint` _spline 1 _returnvalue "Local" true))

(fn `SetSplineTangents`
  (for _index (range (+ (- (`SplineComponent.GetNumberOfSplinePoints` (`self.Spline`)) -1) 1))
    (`self.SetSplinePointTangentLength` _index)))

(fn `UserConstructionScript`)