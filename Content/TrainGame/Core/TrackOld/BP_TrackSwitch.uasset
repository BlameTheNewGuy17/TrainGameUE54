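; Track switch piece for the train game, sitting in the TrackOld folder, that shapes two splines into a straight path and a curved branch.
; AssignSplineCurves reuses or creates the second spline component, then branches on SwitchType, with only Left wired to SetupStandard.
; SetupStandard gives both splines the same Length, with zero curvature on the main and Curve degrees on the second.
; The construction script only calls its parent, and the event graph is inactive.
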(fn `AddSpline`
  (params (InputPin :type "SplineComponent Object Reference"))
  (returns (SplineRef :type "SplineComponent Object Reference"))
  (`/Engine/EditorBlueprintResources/StandardMacros.IsValid` InputPin
    (:`Is Valid`
      (return InputPin))
    (:`Is Not Valid`
      (bind _returnvalue (`AddComponent|NODE_AddSplineComponent-0`))
      (bind _output_get (set `self.Spline2` _returnvalue))
      (return _output_get))))

(fn `AssignSplineCurves`
  (bind _splineref (`self.AddSpline` (`self.Spline2`)))
  (set `self.Spline2` _splineref)
  (switch `/Game/TrainGame/Core/TrackOld/ESwitchType` (`self.SwitchType`)
    (:`NewEnumerator0`
      (`self.SetupStandard`))))

(fn `SetupStandard`
  (`self.SetSplineCurve` (`self.Spline`) (`self.Length`))
  (`self.SetSplineCurve` (`self.Spline2`) (`self.Length`) (`self.Curve`)))

(fn `UserConstructionScript`
  (`parent.UserConstructionScript`))