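; BP_RollingStock is a train rolling stock actor meant to be positioned along track through the track manager.
; Construction generates two bogie meshes spaced by Wheelbase on Body, each with two child meshes.
; BeginPlay caches the tagged BP_TrackManager, and Tick calls SolveFromFront to query a track-distance transform.
; The solve is unfinished: that transform goes unused, Tick passes no coupler state, and SolveFromRear and save initialization are stubs.
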(event `self.ReceiveBeginPlay`
  (bind _outactors (`GameplayStatics.GetAllActorsOfClassWithTag` "/Game/TrainGame/Core/Track/BP_TrackManager.BP_TrackManager_C" "TrackManager"))
  (set `self.TrackManagerRef` (`|GetArrayItem` _outactors)))

(event `self.ReceiveTick`
  (params (DeltaSeconds :type "Float (single-precision)"))
  (`self.SolveFromFront` (struct)))

(event `/Game/TrainGame/Core/RollingStock/BPI_RollingStock.InitializeFromSave`
  (params (CarSaveData :type "/Game/TrainGame/Core/RollingStock/Struct_RollingStockData Structure")))

(fn `EnablePlayerCollision`
  (`PrimitiveComponent.SetCollisionProfileName` (`self.Body`) "BlockAllDynamic" true))

(fn `GenerateBogies`
  (params (Count :type Integer))
  (bind _wheelbase (`self.Wheelbase`))
  (`/Game/TrainGame/Core/ProcFuncs.Delete and Clear Actor Component Array` (`self.Bogies`))
  (for _index (range Count)
    (bind _returnvalue (`AddComponent|NODE_AddStaticMeshComponent-0` :`RelativeTransform` (`KismetMathLibrary.MakeTransform` (`KismetMathLibrary.MakeVector` (- (* _index _wheelbase) (/ _wheelbase 2.0))))))
    (`SceneComponent.K2_AttachToComponent` _returnvalue (`self.Body`) "None" "KeepRelative" "KeepRelative" "KeepRelative" true)
    (`KismetArrayLibrary.Array_Add` (`self.Bogies`) _returnvalue)
    (bind _returnvalue_2 (`AddComponent|NODE_AddStaticMeshComponent-1` :`RelativeTransform` (`KismetMathLibrary.MakeTransform` (80.0 0.0 -40.0))))
    (`SceneComponent.K2_AttachToComponent` _returnvalue_2 _returnvalue "None" "KeepRelative" "KeepRelative" "KeepRelative" true)
    (bind _returnvalue_3 (`AddComponent|NODE_AddStaticMeshComponent-2` :`RelativeTransform` (`KismetMathLibrary.MakeTransform` (-80.0 0.0 -40.0))))
    (`SceneComponent.K2_AttachToComponent` _returnvalue_3 _returnvalue "None" "KeepRelative" "KeepRelative" "KeepRelative" true))
  (return))

(fn `GetRollingStockID`
  (returns (RollingStockID :type Name))
  (return (`self.RollingStockID`)))

(fn `SolveFromFront`
  (params (InputCouplerState :type "/Game/TrainGame/Core/RollingStock/Struct_CouplerState Structure"))
  (returns (OutputCouplerState :type "/Game/TrainGame/Core/RollingStock/Struct_CouplerState Structure"))
  (bind (_trackid _distancealongtrack) (break `/Game/TrainGame/Core/RollingStock/Struct_CouplerState` InputCouplerState))
  (message `/Game/TrainGame/Core/Track/BPI_TrackManagerInterface.GetTransformAtTrackDistance` (`self.TrackManagerRef`) _trackid _distancealongtrack))

(fn `SolveFromRear`
  (params (InputCouplerState :type "/Game/TrainGame/Core/RollingStock/Struct_CouplerState Structure"))
  (returns (OutputCouplerState :type "/Game/TrainGame/Core/RollingStock/Struct_CouplerState Structure"))
  (return))

(fn `UserConstructionScript`
  (`self.GenerateBogies` 2))