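; Physics-driven rolling stock actor that procedurally assembles a rail car from a body, trucks and wheels in its construction script.
; Setup applies a dynamic paint material to the body, then adds simulated truck meshes at suffix-matched body sockets and wheels at matching truck sockets.
; Each added mesh gets a physics constraint to its parent, with angular limits from truck or wheel settings.
; Powered propulsion is unwired, and the component cleanup function is empty.
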(event `self.ReceiveBeginPlay`
  (`KismetSystemLibrary.Delay` 3.0))

(event `self.ReceiveTick`
  (params (DeltaSeconds :type "Float (single-precision)")))

(fn `Add MeshesToSockets`
  (params (Parent :type "StaticMeshComponent Object Reference") (SocketSuffixList :type "Array of String") (NewMesh :type "StaticMesh Object Reference") (ConstraintSettings :type "/Game/TrainGame/Core/PhysRollingStock/Physics/Struct_ConstraintSettings Structure"))
  (locals (Local_MatchingSuffix :type Boolean :default false))
  ;[1 1 1] For each socket found we check it against a list of strings to see if we find one with a matching suffix
  (for _array_element (`SceneComponent.GetAllSocketNames` Parent)
    (set `local.Local_MatchingSuffix` false)
    (for _array_element_2 SocketSuffixList
      (if (`KismetStringLibrary.EndsWith` (`KismetStringLibrary.Conv_NameToString` _array_element) _array_element_2)
        (set `local.Local_MatchingSuffix` true)
        (break)))
    (if (`local.Local_MatchingSuffix`)
      (`self.AddConstrainedMesh` Parent _array_element (`KismetMathLibrary.MakeTransform` (0.0 0.0 0.0)) NewMesh ConstraintSettings))))

(fn `AddConstrainedMesh`
  (params (Parent :type "MeshComponent Object Reference") (SocketName :type Name :default "None") (Transform :type "Transform Structure") (NewMesh :type "StaticMesh Object Reference") (ConstraintSettings :type "/Game/TrainGame/Core/PhysRollingStock/Physics/Struct_ConstraintSettings Structure"))
  (bind ((`AngularTypes_21_4ED7C0A240D77A8BA4A9BFA01F2257B7` _angulartypes) (`Limits_20_10E3CBB84602EBC366E028A7DCCAF349` _limits)) (break `/Game/TrainGame/Core/PhysRollingStock/Physics/Struct_ConstraintSettings` ConstraintSettings))
  (bind _outputpin (`self.AttachMeshToComponent` Parent SocketName Transform NewMesh))
  (bind _outputpin_2 (`self.AttachConstraintToComponent` Parent SocketName Transform))
  (`self.SetConstraintSettings` _outputpin_2 (make `/Game/TrainGame/Core/PhysRollingStock/Physics/Struct_ConstraintSettings` :`Component1` Parent :`Component2` _outputpin :`AngularTypes` _angulartypes :`Limits` _limits)))

(fn `AddWheelMeshes`
  (for _array_element (`self.Meshes`)
    (if (== (`StaticMeshComponent.StaticMesh` _array_element) (`self.TruckMeshDefault`))
      (`self.Add MeshesToSockets` _array_element (`|MakeArray` "00" "01") (`self.WheelMeshDefault`) (`self.WheelConstraintSettings`)))))

(fn `AttachConstraintToComponent`
  (params (Parent :type "SceneComponent Object Reference") (SocketName :type Name :default "None") (Transform :type "Transform Structure (by ref)"))
  (returns (OutputPin :type "PhysicsConstraintComponent Object Reference"))
  (bind _outputpin (`self.CreateAndRegisterConstraint` (`self.CheckUseSocketTransform` Parent SocketName Transform)))
  (`SceneComponent.K2_AttachToComponent` _outputpin Parent SocketName "KeepRelative" "KeepRelative" "KeepRelative" false)
  (return _outputpin))

(fn `AttachMeshToComponent`
  (params (Parent :type "SceneComponent Object Reference") (SocketName :type Name :default "None") (Transform :type "Transform Structure (by ref)") (NewMesh :type "StaticMesh Object Reference"))
  (returns (OutputPin :type "StaticMeshComponent Object Reference"))
  (bind _outputpin (`self.CreateAndRegisterPhysMesh` (`self.CheckUseSocketTransform` Parent SocketName Transform) NewMesh))
  (`SceneComponent.K2_AttachToComponent` _outputpin Parent SocketName "KeepRelative" "KeepRelative" "KeepRelative" true)
  (return _outputpin))

(fn `CheckDynamicMaterialInstance`
  (returns (MaterialRef :type "MaterialInstanceDynamic Object Reference"))
  (`/Engine/EditorBlueprintResources/StandardMacros.IsValid` (`self.DynMatInst`)
    (:`Is Valid`
      _)
    (:`Is Not Valid`
      (bind _returnvalue (`KismetMaterialLibrary.CreateDynamicMaterialInstance` "/Game/TrainGame/MaterialLibrary/RollingStock/MI_Flatcar.MI_Flatcar"))
      (bind _output_get (set `self.DynMatInst` _returnvalue))))
  (return _output_get))

(fn `CheckUseSocketTransform`
  (params (Parent :type "SceneComponent Object Reference") (SocketName :type Name) (Transform :type "Transform Structure (by ref)"))
  (returns (ReturnTransform :type "Transform Structure"))
  (return (`KismetMathLibrary.SelectTransform` Transform (`SceneComponent.GetSocketTransform` Parent SocketName "RTS_ParentBoneSpace") (== SocketName "None"))))

(fn `CreateAndRegisterConstraint`
  (params (RelativeTransform :type "Transform Structure"))
  (returns (OutputPin :type "PhysicsConstraintComponent Object Reference"))
  (bind _returnvalue (`AddComponent|NODE_AddPhysicsConstraintComponent-0` :`RelativeTransform` RelativeTransform))
  (`KismetArrayLibrary.Array_Add` (`self.Constraints`) _returnvalue)
  (return _returnvalue))

(fn `CreateAndRegisterPhysMesh`
  (params (RelativeTransform :type "Transform Structure") (NewMesh :type "StaticMesh Object Reference"))
  (returns (OutputPin :type "StaticMeshComponent Object Reference"))
  (bind _returnvalue (`AddComponent|NODE_AddStaticMeshComponent-2` :`bManualAttachment` true :`RelativeTransform` RelativeTransform))
  (`KismetArrayLibrary.Array_Add` (`self.Meshes`) _returnvalue)
  (`StaticMeshComponent.SetStaticMesh` _returnvalue NewMesh)
  (`PrimitiveComponent.SetSimulatePhysics` _returnvalue true)
  (return _returnvalue))

(fn `CreateBogies`
  (`/Game/TrainGame/Core/ProcFuncs.Delete and Clear Actor Component Array` (`self.Meshes`))
  (`/Game/TrainGame/Core/ProcFuncs.Delete and Clear Actor Component Array` (`self.Constraints`))
  (`self.Add MeshesToSockets` (`self.Body`) (`|MakeArray` "TruckFront" "TruckRear") (`self.TruckMeshDefault`) (`self.TruckConstraintSettings`))
  (`self.AddWheelMeshes`))

(fn `Delete and Clear Actor Component Array`
  (params (Array :type "Array of ActorComponent Object Reference")))

(fn `SetConstraintSettings`
  (params (ConstraintRef :type "PhysicsConstraintComponent Object Reference") (Settings :type "/Game/TrainGame/Core/PhysRollingStock/Physics/Struct_ConstraintSettings Structure") (IsTruck :type Boolean))
  (`PhysicsConstraintComponent.SetDisableCollision` ConstraintRef `Settings_bDisableCollision?_1_C27F218B4D361EE107DAD48074078D44`)
  (`PhysicsConstraintComponent.SetConstrainedComponents` ConstraintRef Settings_Component1_9_EBD0EB894A0C9A59BC7E0E80F1445124 "None" Settings_Component2_10_366CD29B4C2032BDBF4DCA83F01D7049 "None")
  (`PhysicsConstraintComponent.SetAngularTwistLimit` ConstraintRef (cast `EAngularConstraintMotion` (`|GetArrayItem` Settings_AngularTypes_21_4ED7C0A240D77A8BA4A9BFA01F2257B7)) (`|GetArrayItem` Settings_Limits_20_10E3CBB84602EBC366E028A7DCCAF349))
  (`PhysicsConstraintComponent.SetAngularSwing2Limit` ConstraintRef (cast `EAngularConstraintMotion` (`|GetArrayItem` Settings_AngularTypes_21_4ED7C0A240D77A8BA4A9BFA01F2257B7 1)) (`|GetArrayItem` Settings_Limits_20_10E3CBB84602EBC366E028A7DCCAF349 1))
  (`PhysicsConstraintComponent.SetAngularSwing1Limit` ConstraintRef (cast `EAngularConstraintMotion` (`|GetArrayItem` Settings_AngularTypes_21_4ED7C0A240D77A8BA4A9BFA01F2257B7 2)) (`|GetArrayItem` Settings_Limits_20_10E3CBB84602EBC366E028A7DCCAF349 2)))

(fn `Setup`
  (`|ExecutionSequence`
    (:`then_0`
      ;[1 1 1] Dynamic Material setup for body paint
      (`self.CheckDynamicMaterialInstance`)
      (`PrimitiveComponent.SetMaterial` (`self.Body`) 0 (`self.DynMatInst`))
      (`MaterialInstanceDynamic.SetVectorParameterValue` (`self.DynMatInst`) "Color" (`self.PaintColor1`)))
    (:`then_1`
      ;[1 1 1] Procedural Mesh and Constraint setup
      (`StaticMeshComponent.SetStaticMesh` (`self.Body`) (`self.BodyMeshDefault`)))
    (:`then_2`
      (`self.CreateBogies`))))

(fn `UserConstructionScript`
  (`self.Setup`))